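; BP_Alien is an enemy that chases the player and fires projectiles once its PawnSensing component sees a pawn.
; The sighting sets IsSeenPlayer, which this graph never clears, and starts an AI MoveTo toward the player character.
; While the flag is set, a Delay on Tick spaces shots roughly three seconds apart, spawning a scaled-down BP_Projectile at Arrow1's location and rotation.
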(event `self.ReceiveTick`
  (params (DeltaSeconds :type "Float (single-precision)"))
  (bind (_returnvalue_location _returnvalue_rotation) (`KismetMathLibrary.BreakTransform` (`SceneComponent.K2_GetComponentToWorld` (`self.Arrow1`))))
  (if (`self.IsSeenPlayer`)
    (`KismetSystemLibrary.Delay` 3.0)
    (`|SpawnActorFromClass` "/Game/Blueprints/Enemis/BP_Projectile.BP_Projectile_C" (`KismetMathLibrary.MakeTransform` _returnvalue_location _returnvalue_rotation (0.25 0.25 0.25)) "Undefined" "MultiplyWithRoot" null null)))

(event `self.PawnSensing.OnSeePawn`
  (params (Pawn :type "Pawn Object Reference"))
  (set `self.IsSeenPlayer` true)
  (`self.FollowPlayer`))

(event `FollowPlayer`
  (if (`self.IsSeenPlayer`)
    (`|AIMoveTo` self (0.0 0.0 0.0) (`GameplayStatics.GetPlayerCharacter` 0))))

(fn `UserConstructionScript`)