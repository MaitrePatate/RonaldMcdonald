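; BP_Cochon2 is a pig enemy that patrols along the spline of the BP_PathCochon2 actor found in the level.
; A timeline drives its position and rotation along the spline, with play rate derived from TimeToComplete.
; When the player overlaps DetectPlayer, MoveCochon shortens that time for a speed boost, then re-calls itself, restoring the slow pace after a delay.
; The health-based destroy logic is never executed.
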(event `self.ReceiveBeginPlay`
  ;[0.15 0.1117 0.009644 0.5] Patrouille cochon
  (bind _returnvalue (`GameplayStatics.GetActorOfClass` "/Game/Blueprints/Environement/CheminsCochons/BP_PathCochon2.BP_PathCochon2_C"))
  (set `self.PathCochon` _returnvalue)
  (`self.MoveCochon`))

(event `MoveCochon`
  (bind _pathcochon (`self.PathCochon`))
  ;[0.105 0.7396 0.6286 0.5] Boost de speed
  (if (`self.player`)
    (`KismetSystemLibrary.PrintString` "222222")
    (bind _output_get (set `self.TimeToComplete` 5.0))
    (set `self.player` false)
    (`self.MoveCochon`)
    (else
      (`KismetSystemLibrary.Delay` 2.0)
      (bind _output_get_2 (set `self.TimeToComplete` 20.0))))
  ;[0.15 0.1117 0.009644 0.5] Patrouille cochon
  (`TimelineComponent.SetPlayRate` (`self.TimeCochon`) (/ 1.0 _output_get))
  (bind (_direction _movetrack) (`Timeline|TimeCochon`)
    (:`Update`
      (bind _returnvalue (`KismetMathLibrary.Lerp` 0.0 (`SplineComponent.GetSplineLength` (`/Game/Blueprints/Environement/CheminsCochons/BP_PathCochon2.Spline` (`self.PathCochon`))) _movetrack))
      (`self.K2_SetActorTransform` (`KismetMathLibrary.MakeTransform` (`SplineComponent.GetLocationAtDistanceAlongSpline` (`/Game/Blueprints/Environement/CheminsCochons/BP_PathCochon2.Spline` _pathcochon) _returnvalue "World") (`SplineComponent.GetRotationAtDistanceAlongSpline` (`/Game/Blueprints/Environement/CheminsCochons/BP_PathCochon2.Spline` _pathcochon) _returnvalue "Local"))))))

(event `self.DetectPlayer.OnComponentBeginOverlap`
  (params (OverlappedComponent :type "PrimitiveComponent Object Reference") (OtherActor :type "Actor Object Reference") (OtherComp :type "PrimitiveComponent Object Reference") (OtherBodyIndex :type Integer) (bFromSweep :type Boolean) (SweepResult :type "HitResult Structure (by ref)"))
  ;[0.105 0.7396 0.6286 0.5] Boost de speed
  (if (== (`GameplayStatics.GetPlayerCharacter` 0) OtherActor)
    (`KismetSystemLibrary.PrintString` "Hello")
    (set `self.player` true)
    (`self.MoveCochon`)))

(fn `UserConstructionScript`)