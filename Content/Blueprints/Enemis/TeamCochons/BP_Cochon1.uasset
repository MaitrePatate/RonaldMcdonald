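; Enemy pig actor that patrols along a spline path in the level.
; On BeginPlay it finds the BP_PathCochon1 actor by class, then plays a timeline with its rate scaled by TimeToComplete.
; Each timeline update maps the MoveTrack alpha to a distance along the spline and sets the pig's transform, taking location in world space and rotation in spline-local space.
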(event `self.ReceiveBeginPlay`
  ;[0.15 0.1117 0.009644 0.5] Patrouille cochon
  (bind _returnvalue (`GameplayStatics.GetActorOfClass` "/Game/Blueprints/Environement/CheminsCochons/BP_PathCochon1.BP_PathCochon1_C"))
  (set `self.SplineRef` _returnvalue)
  (`self.MoveCochon`))

(event `MoveCochon`
  (bind _splineref (`self.SplineRef`))
  ;[0.15 0.1117 0.009644 0.5] Patrouille cochon
  (`TimelineComponent.SetPlayRate` (`self.TimeCochon`) (/ 1.0 (`self.TimeToComplete`)))
  (bind (_direction _movetrack) (`Timeline|TimeCochon`)
    (:`Update`
      (bind _returnvalue (`KismetMathLibrary.Lerp` 0.0 (`SplineComponent.GetSplineLength` (`/Game/Blueprints/Environement/CheminsCochons/BP_PathCochon1.Spline` (`self.SplineRef`))) _movetrack))
      (`self.K2_SetActorTransform` (`KismetMathLibrary.MakeTransform` (`SplineComponent.GetLocationAtDistanceAlongSpline` (`/Game/Blueprints/Environement/CheminsCochons/BP_PathCochon1.Spline` _splineref) _returnvalue "World") (`SplineComponent.GetRotationAtDistanceAlongSpline` (`/Game/Blueprints/Environement/CheminsCochons/BP_PathCochon1.Spline` _splineref) _returnvalue "Local"))))))

(fn `UserConstructionScript`)